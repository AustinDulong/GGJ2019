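; Player controller that switches control between three characters: Craig_Digger, Judy_grapler and Danny_dino.
; Pressing the 1 key advances a PlayerCharacter index that wraps to 0 after 3.
; Releasing it possesses the first level actor of the matching class, found with GetAllActorsOfClass.
; Index 3 has no matching case, so that step of the cycle leaves possession unchanged.
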(event EventBeginPlay)

(event EventTick
  (params (DeltaSeconds :type Float%20%28single-precision%29)))

(event Input|KeyboardEvents|1
  (params (Key :type Key%20Structure))
  (:Pressed
    (if (== (Variables|Default|GetPlayer_Character) 3)
      (Variables|Default|SetPlayer_Character 0)
      (else
        (Variables|Default|SetPlayer_Character (+ (Variables|Default|GetPlayer_Character) 1)))))
  (:Released
    (switch int (Variables|Default|GetPlayer_Character)
      (:0
        (bind _outactors (Actor|GetAllActorsOfClass "/Game/GameJam2019/Characters/Craig_Digger.Craig_Digger_C"))
        (Pawn|Possess (Utilities|Array|Get(acopy) _outactors)))
      (:1
        (bind _outactors_2 (Actor|GetAllActorsOfClass "/Game/GameJam2019/Characters/Judy_grapler.Judy_grapler_C"))
        (Pawn|Possess (Utilities|Array|Get(acopy) _outactors_2)))
      (:2
        (bind _outactors_3 (Actor|GetAllActorsOfClass "/Game/GameJam2019/Characters/Danny_dino.Danny_dino_C"))
        (Pawn|Possess (Utilities|Array|Get(acopy) _outactors_3))))))

(fn ConstructionScript)